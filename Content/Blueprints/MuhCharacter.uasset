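; MuhCharacter is a player character with look and movement input, a chargeable projectile attack and a parry probe.
; Holding Fire runs a timeline, and releasing it spawns a MuhProjectile ahead of the camera, aimed along control rotation and scaled up by the timeline value.
; Parry runs a debug-drawn box trace for WorldDynamic objects in front of the character, but its result is not yet used.
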(event Input|ActionEvents|InputActionFire
  (params (Key :type Key%20Structure))
  (:Pressed
    (bind _newtrack_0 (Timeline|ChargeTimeline PlayFromStart)))
  (:Released
    (Game|SpawnActorfromClass "/Game/Blueprints/MuhProjectile.MuhProjectile_C" (Math|Transform|MakeTransform (+ (Transformation|GetActorLocation) (* (Math|Vector|GetForwardVector (Variables|Default|GetCamera)) 5e+01)) (Pawn|GetControlRotation :!class /Script/Engine.Pawn) (Math|Vector|Lerp(Vector) "1.000000,1.000000,1.000000" "10.000000,10.000000,10.000000" _newtrack_0)) "Undefined" 0 0)))

(event Input|ActionEvents|InputActionParry
  (params (Key :type Key%20Structure))
  (bind _returnvalue (Transformation|GetActorLocation))
  (bind _returnvalue_2 (Transformation|GetActorForwardVector))
  (bind _returnvalue_3 (* _returnvalue_2 2e+02))
  (bind _returnvalue_4 (+ _returnvalue _returnvalue_3))
  (:Pressed
    (Class|KismetSystemLibrary|BoxTraceSingleforObjects _returnvalue_4 (+ _returnvalue_4 "1.000000, 0,0.000000") "100.000000,100.000000,100.000000" "0, 0, 0" (Utilities|Array|MakeArray "ObjectTypeQuery2") false 0 "ForDuration" true "(R=1.000000,G=0.000000,B=0.000000,A=1.000000)" "(R=0.000000,G=1.000000,B=0.000000,A=1.000000)" 1.0)))

(event Input|AxisEvents|InputAxisLookUp
  (params (AxisValue :type Float%20%28single-precision%29))
  ;[1 1 1] Look and Move
  (Pawn|Input|AddControllerPitchInput AxisValue))

(event Input|AxisEvents|InputAxisTurn
  (params (AxisValue :type Float%20%28single-precision%29))
  ;[1 1 1] Look and Move
  (Pawn|Input|AddControllerYawInput AxisValue))

(event Input|AxisEvents|InputAxisMoveForward
  (params (AxisValue :type Float%20%28single-precision%29))
  ;[1 1 1] Look and Move
  (Pawn|Input|AddMovementInput (Transformation|GetActorForwardVector) AxisValue false))

(event Input|AxisEvents|InputAxisMoveRight
  (params (AxisValue :type Float%20%28single-precision%29))
  ;[1 1 1] Look and Move
  (Pawn|Input|AddMovementInput (Transformation|GetActorRightVector) AxisValue false))

(fn ConstructionScript)